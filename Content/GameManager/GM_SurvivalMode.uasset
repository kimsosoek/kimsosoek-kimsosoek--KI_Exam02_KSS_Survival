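; Survival game mode that spawns enemies and MP pickups around the player until a countdown ends.
; Looping timers spawn a random BP_EnemyCharacter or BP_Enemy_Ranged, plus MP potions, at random navigable points near the player.
; UpdateGameTimer decrements the remaining time, then disables input and shows WBP_Scoreboard with a UI-only cursor.
; No timer is cleared, so spawning and scoreboard creation repeat after time runs out.
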(event Custom|SpawnEnemyWave
  (bind _returnvalue (Math|Rotator|MakeRotator 0.0 0.0 0.0))
  ;[0.15 0.15 0.15 0.5] 적 스폰
  (bind _randomlocation (Class|NavigationSystemV1|GetRandomLocationinNavigableRadius (Transformation|GetActorLocation (Game|GetPlayerCharacter 0)) 3e+03 0 "/Script/AIModule.NavFilter_AIControllerDefault"))
  (if true
    (switch int (Math|Random|RandomIntegerinRange 0 1)
      (:Default
        (Game|SpawnActorfromClass "/Game/Character/BP_Enemy_Ranged.BP_Enemy_Ranged_C" (Math|Transform|MakeTransform _randomlocation _returnvalue "1.000000,1.000000,1.000000") "Undefined" "MultiplyWithRoot" 0 0))
      (:0
        (Game|SpawnActorfromClass "/Game/Character/BP_EnemyCharacter.BP_EnemyCharacter_C" (Math|Transform|MakeTransform _randomlocation _returnvalue "1.000000,1.000000,1.000000") "Undefined" "MultiplyWithRoot" 0 0)))))

(event Custom|SpawnMPPotion
  ;[0.15 0.15 0.15 0.5] 뮬약 스폰
  (bind _randomlocation (Class|NavigationSystemV1|GetRandomLocationinNavigableRadius (Transformation|GetActorLocation (Game|GetPlayerCharacter 0)) 3e+03 0 "/Script/AIModule.NavFilter_AIControllerDefault"))
  (Game|SpawnActorfromClass "/Game/Actor/BP_MP_PIckUP.BP_MP_PIckUP_C" (Math|Transform|MakeTransform _randomlocation (Math|Rotator|MakeRotator 0.0 0.0 0.0) "1.000000,1.000000,1.000000") "Undefined" "MultiplyWithRoot" 0 0))

(event EventBeginPlay
  (Utilities|FlowControl|Sequence
    (:then_0
      ;[0.15 0.15 0.15 0.5] 적 스폰
      (Utilities|Time|SetTimerbyEvent (delegate Custom|SpawnEnemyWave) 0.5 true)
      (Utilities|Time|SetTimerbyFunctionName 0 "UpdateGameTimer" 1.0 true))
    (:then_1
      ;[0.15 0.15 0.15 0.5] 뮬약 스폰
      (Utilities|Time|SetTimerbyEvent (delegate Custom|SpawnMPPotion) 0.5 true)
      (Utilities|Time|SetTimerbyFunctionName 0 "UpdateGameTimer" 1.0 true))))

(fn ConstructionScript)

(fn GetPlayerRef
  (bind _returnvalue (Game|GetPlayerCharacter 0))
  (Development|PrintString (Utilities|GetDisplayName _returnvalue))
  (bind _asbp_player_character (Utilities|Casting|CastToBP_PlayerCharacter _returnvalue)
    (:then
      (return _asbp_player_character))
    (:CastFailed
      (Development|PrintString "형변환실패"))))

(fn UpdateGameTimer
  (bind _returnvalue (Game|GetPlayerController 0))
  (Variables|Default|SetGameTimeRemaining (- (Variables|Default|GetGameTimeRemaining) 1.0))
  (if (<= (Variables|Default|GetGameTimeRemaining) 0.0)
    (Input|DisableInput _returnvalue 0)
    (bind _returnvalue_2 (UserInterface|CreateWidget "/Game/GameManager/WBP_Scoreboard.WBP_Scoreboard_C"))
    (UserInterface|Viewport|AddtoViewport _returnvalue_2 0)
    (Variables|/Script/Engine.PlayerController|SetbShowMouseCursor _returnvalue true)
    (Input|SetInputModeUIOnly _returnvalue 0 "DoNotLock" false)))