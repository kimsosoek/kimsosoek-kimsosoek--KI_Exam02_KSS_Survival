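; Player character Blueprint for a shooter, handling movement, aiming, combat, HP/MP/booster stats and the main HUD.
; Firing requires aiming, which zooms FOV by timeline; a camera trace orients bullets spawned at the rifle muzzle, with a timer repeating shots.
; Dashing spends booster, regenerated on Tick, to raise walk speed, while the skill spends MP to launch a grenade.
; Damage shakes the camera and, at zero HP, triggers ragdoll and the game-over screen.
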(event Custom|Event_Fire
  (bind _camera (Variables|Default|GetCamera))
  (bind _riflemesh (Variables|Default|GetRifleMesh))
  (bind _returnvalue (Transformation|GetWorldLocation _camera))
  (bind _returnvalue_2 (Transformation|GetSocketLocation _riflemesh "Muzzle"))
  (bind (_outhit _returnvalue_3) (Collision|LineTraceByChannel _returnvalue (+ _returnvalue (* (Math|Vector|GetForwardVector _camera) 1e+04)) "TraceTypeQuery1" false (Utilities|Array|MakeArray self) "None"))
  (Game|SpawnActorfromClass "/Game/Actor/BP_Projectile_Bullet.BP_Projectile_Bullet_C" (Math|Transform|MakeTransform _returnvalue_2 (Math|Rotator|FindLookatRotation _returnvalue_2 (select _returnvalue_3 (.Location (Collision|BreakHitResult _outhit)) (.TraceEnd (Collision|BreakHitResult _outhit)))) "1.000000,1.000000,1.000000") "AlwaysSpawn" "MultiplyWithRoot" 0 0)
  (Components|Activation|Activate (Variables|Default|GetNiagara) false)
  (bind _returnvalue_4 (Utilities|Time|SetTimerbyEvent (delegate Custom|Event_Fire) (Variables|Default|GetFireRate) true))
  (Variables|Default|SetFireTimerHandle _returnvalue_4)
  (Components|Activation|Deactivate (Variables|Default|GetNiagara)))

(event Custom|DashActivate
  (Variables|/Script/Engine.CharacterMovementComponent|SetMaxWalkSpeed (Variables|Character|GetCharacterMovement) (Variables|Default|GetRunSpeed)))

(event Custom|DashDeactivate
  (Variables|/Script/Engine.CharacterMovementComponent|SetMaxWalkSpeed (Variables|Character|GetCharacterMovement) (Variables|Default|GetWalkspeed)))

(event Input|EnhancedActionEvents|EnhancedInputActionIA_Move
  (params (ActionValue :type Vector%202D%20Structure) (ElapsedSeconds :type Float%20%28double-precision%29) (TriggeredSeconds :type Float%20%28double-precision%29) (InputAction :type Input%20Action%20Object%20Reference :default "/Game/Input/IA_Move.IA_Move"))
  ;[0.15 0.15 0.15 0.5] 움직임
  (Utilities|FlowControl|Sequence
    (:then_0
      (Pawn|Input|AddMovementInput (Math|Vector|GetForwardVector (Pawn|GetControlRotation :!class /Script/Engine.Pawn)) (.x ActionValue) false))
    (:then_1
      (Pawn|Input|AddMovementInput (Math|Vector|GetRightVector (Pawn|GetControlRotation :!class /Script/Engine.Pawn)) (.y ActionValue) false))))

(event Input|EnhancedActionEvents|EnhancedInputActionIA_Look
  (params (ActionValue :type Vector%202D%20Structure) (ElapsedSeconds :type Float%20%28double-precision%29) (TriggeredSeconds :type Float%20%28double-precision%29) (InputAction :type Input%20Action%20Object%20Reference :default "/Game/Input/IA_Look.IA_Look"))
  (Pawn|Input|AddControllerYawInput (.x ActionValue))
  (Pawn|Input|AddControllerPitchInput (* (.y ActionValue) -1.0)))

(event Input|EnhancedActionEvents|EnhancedInputActionIA_Jump
  (params (ActionValue :type Boolean) (ElapsedSeconds :type Float%20%28double-precision%29) (TriggeredSeconds :type Float%20%28double-precision%29) (InputAction :type Input%20Action%20Object%20Reference :default "/Game/Input/IA_Jump.IA_Jump"))
  (:Started
    (if (not (AI|Components|NavMovement|IsFalling (Variables|Character|GetCharacterMovement)))
      (Character|Jump)))
  (:Canceled
    (Character|StopJumping)))

(event Input|EnhancedActionEvents|EnhancedInputActionIA_Fire
  (params (ActionValue :type Boolean) (ElapsedSeconds :type Float%20%28double-precision%29) (TriggeredSeconds :type Float%20%28double-precision%29) (InputAction :type Input%20Action%20Object%20Reference :default "/Game/Input/IA_Fire.IA_Fire"))
  (:Triggered
    (if (Variables|Default|GetbIsAiming)
      (Animation|PlayAnimMontage "/Game/Animation/AM_IdleFire.AM_IdleFire" 2.0 "None")
      (CallFunction|EventFire)))
  (:Completed
    (Utilities|Time|ClearandInvalidateTimerbyHandle (Variables|Default|GetFireTimerHandle))))

(event Input|EnhancedActionEvents|EnhancedInputActionIA_Dash
  (params (ActionValue :type Boolean) (ElapsedSeconds :type Float%20%28double-precision%29) (TriggeredSeconds :type Float%20%28double-precision%29) (InputAction :type Input%20Action%20Object%20Reference :default "/Game/Input/IA_Dash.IA_Dash"))
  (:Triggered
    (if (> (Variables|Default|GetCurrentBooster) (Variables|Default|GetDashCost))
      (Variables|Default|SetCurrentBooster (- (Variables|Default|GetCurrentBooster) (Variables|Default|GetDashCost)))
      (Timeline|타임라인 Play
        (:Update
          (CallFunction|DashActivate)))
      (else
        (bind _output_get (Variables|Default|SetCurrentBooster (- (Variables|Default|GetCurrentBooster) (Variables|Default|GetDashCost))))
        (CallFunction|DashDeactivate))))
  (:Completed
    (CallFunction|DashDeactivate)))

(event Input|EnhancedActionEvents|EnhancedInputActionIA_Aim
  (params (ActionValue :type Boolean) (ElapsedSeconds :type Float%20%28double-precision%29) (TriggeredSeconds :type Float%20%28double-precision%29) (InputAction :type Input%20Action%20Object%20Reference :default "/Game/Input/IA_Aim.IA_Aim"))
  ;[0.15 0.15 0.15 0.5] 줌
  (:Started
    (Variables|Default|SetbIsAiming true)
    (Variables|/Script/Engine.CharacterMovementComponent|SetbOrientRotationToMovement (Variables|Character|GetCharacterMovement) false)
    (Variables|Default|SetbUseControllerRotationYaw true)
    (bind _zoomalpha (Timeline|AimZoomTimeLine Play)
      (:Update
        (Camera|SetFieldOfView (Variables|Default|GetCamera) (Math|Float|Lerp 1e+02 4e+01 _zoomalpha)))))
  (:Completed
    (Variables|Default|SetbIsAiming false)
    (Variables|/Script/Engine.CharacterMovementComponent|SetbOrientRotationToMovement (Variables|Character|GetCharacterMovement) true)
    (Variables|Default|SetbUseControllerRotationYaw true)
    (Timeline|AimZoomTimeLine Reverse)))

(event Input|EnhancedActionEvents|EnhancedInputActionIA_Skill
  (params (ActionValue :type Boolean) (ElapsedSeconds :type Float%20%28double-precision%29) (TriggeredSeconds :type Float%20%28double-precision%29) (InputAction :type Input%20Action%20Object%20Reference :default "/Game/Input/IA_Skill.IA_Skill"))
  ;[0.15 0.15 0.15 0.5] 폭발물
  (:Started
    (if (>= (Variables|Default|GetCurrentMP) (Variables|Default|GetSkillCost))
      (Variables|Default|SetCurrentMP (- (Variables|Default|GetCurrentMP) (Variables|Default|GetSkillCost)))
      (Game|SpawnActorfromClass "/Game/Actor/BP_Grenade.BP_Grenade_C" (Math|Transform|MakeTransform (Transformation|GetWorldLocation (Variables|Default|GetMuzzle)) (Transformation|GetWorldRotation (Variables|Default|GetCamera)) "1.000000,1.000000,1.000000") "AlwaysSpawn" "MultiplyWithRoot" 0 self 0)
      (Components|Activation|Activate (Variables|Default|GetNiagara) false)
      (Components|Activation|Deactivate (Variables|Default|GetNiagara)))))

(event EventBeginPlay
  (Utilities|FlowControl|Sequence
    (:then_0
      (Variables|Default|SetCurrentHP (Variables|Default|GetMaxHP))
      (Variables|Default|SetCurrentMP (Variables|Default|GetMaxMP))
      (Variables|Default|SetCurrentBooster (Variables|Default|GetMaxBooster))
      (Variables|/Script/Engine.CharacterMovementComponent|SetMaxWalkSpeed (Variables|Character|GetCharacterMovement) (Variables|Default|GetWalkspeed)))
    (:then_1
      (bind _returnvalue (UserInterface|CreateWidget "/Game/GameManager/WBP_MainHUD.WBP_MainHUD_C"))
      (UserInterface|Viewport|AddtoViewport _returnvalue 0))))

(event Game|Damage|EventAnyDamage
  (params (Damage :type Float%20%28single-precision%29) (DamageType :type Damage%20Type%20Object%20Reference) (InstigatedBy :type Controller%20Object%20Reference) (DamageCauser :type Actor%20Object%20Reference))
  (bind _returnvalue (Game|GetPlayerController 0))
  (Camera|PlayWorldCameraShake "/Game/CS_Player_Hit.CS_Player_Hit_C" (Transformation|GetActorLocation) 0.0 2e+03)
  (bind _output_get (Variables|Default|SetCurrentHP (Math|Float|Clamp(Float) (- (Variables|Default|GetCurrentHP) Damage) 0.0 (Variables|Default|GetMaxHP))))
  (if (<= _output_get 0.0)
    (Input|DisableInput (Game|GetPlayerController 0) 0)
    (Collision|SetCollisionEnabled (Variables|Collision|GetCapsuleComponent) "NoCollision")
    (Collision|SetCollisionProfileName (Variables|Character|GetMesh) "Ragdoll" true :!class /Script/Engine.PrimitiveComponent)
    (Physics|SetSimulatePhysics (Variables|Character|GetMesh) true)
    (Utilities|FlowControl|Delay 1.0)
    (bind _returnvalue_2 (UserInterface|CreateWidget "/Game/GameManager/WBP_GameOver.WBP_GameOver_C"))
    (UserInterface|Viewport|AddtoViewport _returnvalue_2 0)
    (Variables|/Script/Engine.PlayerController|SetbShowMouseCursor _returnvalue true)
    (Input|SetInputModeUIOnly _returnvalue _returnvalue_2 "DoNotLock" false)))

(event EventTick
  (params (DeltaSeconds :type Float%20%28single-precision%29))
  ;[0.15 0.15 0.15 0.5] 부스터 충전
  (if (< (Variables|Default|GetCurrentBooster) (Variables|Default|GetMaxBooster))
    (Variables|Default|SetCurrentBooster (Math|Float|Clamp(Float) (+ (* DeltaSeconds (Variables|Default|GetBoosterRegenRate)) (Variables|Default|GetCurrentBooster)) 0.0 (Variables|Default|GetMaxBooster)))))

(fn ConstructionScript)