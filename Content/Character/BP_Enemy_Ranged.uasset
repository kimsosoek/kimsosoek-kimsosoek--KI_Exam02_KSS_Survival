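; Ranged enemy character for survival mode that starts its behavior tree through AIC_Enemy_Ranged on BeginPlay.
; AnyDamage and a separate TakeDamage event both reduce HP, and on death increment the GM_SurvivalMode kill count, stop AI, ragdoll and expire; only TakeDamage sets IsDead.
; Helpers find the player by sphere overlap, flag a lost target and return waypoint locations, though IncreaseWaypointIndex is empty.
; It also carries player-style move and jump input handlers.
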(event Custom|LostTarget
  (Variables|Default|SetbBotLostTarget true))

(event Custom|TakeDamage
  (params (DamageAmount :type Float%20%28double-precision%29))
  (Variables|Default|SetCurrentHP (- (Variables|Default|GetCurrentHP) DamageAmount))
  (if (<= (Variables|Default|GetCurrentHP) 0.0)
    (bind _asgm_survival_mode (Utilities|Casting|CastToGM_SurvivalMode (Game|GetGameMode)))
    (Variables|/Game/GameManager/GM_SurvivalMode.GM_SurvivalMode_C|SetKillCount _asgm_survival_mode (+ (Variables|/Game/GameManager/GM_SurvivalMode.GM_SurvivalMode_C|GetKillCount _asgm_survival_mode) 1))
    (Variables|Default|SetIsDead true)
    (bind _asaic_enemy_ranged (Utilities|Casting|CastToAIC_Enemy_Ranged (Pawn|GetController)))
    (AI|Logic|StopLogic (Variables|/Script/AIModule.AIController|GetBrainComponent _asaic_enemy_ranged) "")
    (Pawn|Components|CharacterMovement|DisableMovement (Variables|Character|GetCharacterMovement))
    (Collision|SetCollisionEnabled (Variables|Collision|GetCapsuleComponent) "NoCollision")
    (Collision|SetCollisionProfileName (Variables|Character|GetMesh) "Ragdoll" true :!class /Script/Engine.PrimitiveComponent)
    (Physics|SetSimulatePhysics (Variables|Character|GetMesh) true)
    (Actor|SetLifeSpan 3.0)))

(event Input|EnhancedActionEvents|EnhancedInputActionIA_Move
  (params (ActionValue :type Vector%202D%20Structure) (ElapsedSeconds :type Float%20%28double-precision%29) (TriggeredSeconds :type Float%20%28double-precision%29) (InputAction :type Input%20Action%20Object%20Reference :default "/Game/Input/IA_Move.IA_Move"))
  ;[0.15 0.15 0.15 0.5] 움직임
  (Utilities|FlowControl|Sequence
    (:then_0
      (Pawn|Input|AddMovementInput (Math|Vector|GetForwardVector (Pawn|GetControlRotation :!class /Script/Engine.Pawn)) (.x ActionValue) false))
    (:then_1
      (Pawn|Input|AddMovementInput (Math|Vector|GetRightVector (Pawn|GetControlRotation :!class /Script/Engine.Pawn)) (.y ActionValue) false))))

(event Input|EnhancedActionEvents|EnhancedInputActionIA_Jump
  (params (ActionValue :type Boolean) (ElapsedSeconds :type Float%20%28double-precision%29) (TriggeredSeconds :type Float%20%28double-precision%29) (InputAction :type Input%20Action%20Object%20Reference :default "/Game/Input/IA_Jump.IA_Jump"))
  (:Triggered
    (Character|Jump))
  (:Canceled
    (Character|StopJumping)))

(event EventBeginPlay
  (Variables|Default|SetCurrentHP (Variables|Default|GetMaxHP))
  (Variables|/Script/Engine.CharacterMovementComponent|SetMaxWalkSpeed (Variables|Character|GetCharacterMovement) (Variables|Default|Get최대%20걷기%20속도))
  (bind _asaic_enemy_ranged (Utilities|Casting|CastToAIC_Enemy_Ranged (Pawn|GetController)))
  (AI|RunBehaviorTree _asaic_enemy_ranged "/Game/AI/BT_Enemy_Ranged.BT_Enemy_Ranged"))

(event EventIncreaseWaypointIndex)

(event Game|Damage|EventAnyDamage
  (params (Damage :type Float%20%28single-precision%29) (DamageType :type Damage%20Type%20Object%20Reference) (InstigatedBy :type Controller%20Object%20Reference) (DamageCauser :type Actor%20Object%20Reference))
  (Variables|Default|SetCurrentHP (Math|Float|Clamp(Float) (- (Variables|Default|GetCurrentHP) Damage) 0.0 (Variables|Default|GetMaxHP)))
  (if (<= (Variables|Default|GetCurrentHP) 0.0)
    (bind _asgm_survival_mode (Utilities|Casting|CastToGM_SurvivalMode (Game|GetGameMode)))
    (Variables|/Game/GameManager/GM_SurvivalMode.GM_SurvivalMode_C|SetKillCount _asgm_survival_mode (+ (Variables|/Game/GameManager/GM_SurvivalMode.GM_SurvivalMode_C|GetKillCount _asgm_survival_mode) 1))
    (bind _asaic_enemy_ranged (Utilities|Casting|CastToAIC_Enemy_Ranged (Pawn|GetController)))
    (AI|Logic|StopLogic (Variables|/Script/AIModule.AIController|GetBrainComponent _asaic_enemy_ranged) "")
    (Pawn|Components|CharacterMovement|DisableMovement (Variables|Character|GetCharacterMovement))
    (Collision|SetCollisionEnabled (Variables|Collision|GetCapsuleComponent) "NoCollision")
    (Collision|SetCollisionProfileName (Variables|Character|GetMesh) "Ragdoll" true :!class /Script/Engine.PrimitiveComponent)
    (Physics|SetSimulatePhysics (Variables|Character|GetMesh) true)
    (Actor|SetLifeSpan 3.0)))

(fn ConstructionScript)

(fn FindTarget
  (bind (_outactors _returnvalue) (Collision|SphereOverlapActors (Transformation|GetActorLocation) (Variables|Default|GetSightRadius) (Utilities|Array|MakeArray "ObjectTypeQuery3") "/Game/Character/BP_PlayerCharacter.BP_PlayerCharacter_C"))
  (if _returnvalue
    (return (Utilities|Array|Get(acopy) _outactors))
    (else
      (return (Utilities|Array|Get(acopy) _outactors)))))

(fn GetWaypointLocation
  (return (Transformation|GetActorLocation (Utilities|Array|Get(acopy) (Variables|Default|GetWaypoints) (Variables|Default|GetWaypointIndex)))))