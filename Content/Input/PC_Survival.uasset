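; PC_Survival is a player controller that sets up input and UI based on the current level when play begins.
; On MAP_MainMenu it creates the main menu widget, shows the cursor and switches to UI-only input focused on that widget.
; On any other level it uses game-only input and hides the cursor.
; Both paths add the IMC_Default Enhanced Input mapping context; Tick is unused.
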(event EventBeginPlay
  (bind _returnvalue (Game|GetPlayerController 0))
  (bind _returnvalue_2 (Game|GetPlayerController 0))
  (bind _returnvalue_3 (Game|GetCurrentLevelName true))
  (if (Utilities|Enum|Equal(Enum) _returnvalue_3 "MAP_MainMenu")
    (bind _returnvalue_4 (UserInterface|CreateWidget "/Game/GameManager/WBP_MainMenu.WBP_MainMenu_C"))
    (UserInterface|Viewport|AddtoViewport _returnvalue_4 0)
    (Variables|Default|SetbShowMouseCursor true)
    (Input|SetInputModeUIOnly _returnvalue_2 _returnvalue_4 "DoNotLock" false)
    (Input|AddMappingContext (PlayerController|LocalPlayerSubsystems|GetEnhancedInputLocalPlayerSubsystem _returnvalue_2) "/Game/Input/IMC_Default.IMC_Default" 0 "(bIgnoreAllPressedKeysUntilRelease=True,bForceImmediately=False,bNotifyUserSettings=False)")
    (else
      (Input|AddMappingContext (PlayerController|LocalPlayerSubsystems|GetEnhancedInputLocalPlayerSubsystem _returnvalue) "/Game/Input/IMC_Default.IMC_Default" 0 "(bIgnoreAllPressedKeysUntilRelease=True,bForceImmediately=False,bNotifyUserSettings=False)")
      (Input|SetInputModeGameOnly _returnvalue false)
      (Variables|Default|SetbShowMouseCursor false))))

(event EventTick
  (params (DeltaSeconds :type Float%20%28single-precision%29)))

(fn ConstructionScript)