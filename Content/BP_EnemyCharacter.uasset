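; BP_EnemyCharacter is an enemy character with health, waypoint patrol data and player detection.
; Health starts at max; AnyDamage subtracts with clamping and a separate TakeDamage event subtracts without it, both destroying the actor at zero or below.
; Helpers expose the current waypoint location, wrap the waypoint index and flag a lost target.
; FindTarget sphere-overlaps for BP_PlayerCharacter pawns within sight radius, returning the first array entry even when none is found.
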(event Custom|TakeDamage
  (params (DamageAmount :type Float%20%28double-precision%29))
  (Variables|Default|SetCurrentHP (- (Variables|Default|GetCurrentHP) DamageAmount))
  (if (<= (Variables|Default|GetCurrentHP) 0.0)
    (Actor|DestroyActor)))

(event Custom|LostTarget
  (Variables|Default|SetbBotLostTarget true))

(event EventBeginPlay
  (Variables|Default|SetCurrentHP (Variables|Default|GetMaxHP)))

(event EventIncreaseWaypointIndex
  (bind _result (Math|Integer|IncrementInt (Variables|Default|GetWaypointIndex))
    (:%20%20
      (Variables|Default|SetWaypointIndex (Math|Integer|%(Integer) _result (Utilities|Array|Length (Variables|Default|GetWaypoints)))))))

(event Game|Damage|EventAnyDamage
  (params (Damage :type Float%20%28single-precision%29) (DamageType :type Damage%20Type%20Object%20Reference) (InstigatedBy :type Controller%20Object%20Reference) (DamageCauser :type Actor%20Object%20Reference))
  (Variables|Default|SetCurrentHP (Math|Float|Clamp(Float) (- (Variables|Default|GetCurrentHP) Damage) 0.0 (Variables|Default|GetMaxHP)))
  (if (<= (Variables|Default|GetCurrentHP) 0.0)
    (Actor|DestroyActor)))

(fn ConstructionScript)

(fn FindTarget
  (bind (_outactors _returnvalue) (Collision|SphereOverlapActors (Transformation|GetActorLocation) (Variables|Default|GetSightRadius) (Utilities|Array|MakeArray "ObjectTypeQuery3") "/Game/BP_PlayerCharacter.BP_PlayerCharacter_C"))
  (if _returnvalue
    (return (Utilities|Array|Get(acopy) _outactors))
    (else
      (return (Utilities|Array|Get(acopy) _outactors)))))

(fn GetWaypointLocation
  (return (Transformation|GetActorLocation (Utilities|Array|Get(acopy) (Variables|Default|GetWaypoints) (Variables|Default|GetWaypointIndex)))))