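; Survival game mode that continuously spawns enemies around the player.
; A looping one-second timer started on BeginPlay spawns a single BP_EnemyCharacter at a random navigable point within a radius of the player character, with no wave count or cap.
; A GetPlayerRef helper returns the player cast to BP_PlayerCharacter, printing debug text with its name and on cast failure.
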(event Custom|SpawnEnemyWave
  (bind _randomlocation (Class|NavigationSystemV1|GetRandomLocationinNavigableRadius (Transformation|GetActorLocation (Game|GetPlayerCharacter 0)) 3e+03 0 "/Script/AIModule.NavFilter_AIControllerDefault"))
  (Game|SpawnActorfromClass "/Game/BP_EnemyCharacter.BP_EnemyCharacter_C" (Math|Transform|MakeTransform _randomlocation (Math|Rotator|MakeRotator 0.0 0.0 0.0) "1.000000,1.000000,1.000000") "Undefined" "MultiplyWithRoot" 0 0))

(event EventBeginPlay
  (Utilities|FlowControl|Sequence
    (:then_0
      (Utilities|Time|SetTimerbyEvent (delegate Custom|SpawnEnemyWave) 1.0 true))))

(event EventTick
  (params (DeltaSeconds :type Float%20%28single-precision%29)))

(fn ConstructionScript)

(fn GetPlayerRef
  (bind _returnvalue (Game|GetPlayerCharacter 0))
  (Development|PrintString (Utilities|GetDisplayName _returnvalue))
  (bind _asbp_player_character (Utilities|Casting|CastToBP_PlayerCharacter _returnvalue)
    (:then
      (return _asbp_player_character))
    (:CastFailed
      (Development|PrintString "형변환실패"))))