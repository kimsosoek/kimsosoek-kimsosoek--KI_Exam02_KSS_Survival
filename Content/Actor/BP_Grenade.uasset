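; Grenade projectile actor that explodes on its first bounce, as reported by its ProjectileMovement component.
; The explosion spawns a big fire-and-smoke Niagara effect at the actor's location and applies radial damage using its damage and radius variables, sparing the grenade's owner.
; It also activates its own Niagara component, then deactivates it in the same call just before destroying itself.
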(event OnProjectileBounce(ProjectileMovement)
  (params (ImpactResult :type Hit%20Result%20Structure%20%28by%20ref%29) (ImpactVelocity :type Vector%20%28by%20ref%29 :default "0, 0, 0"))
  (CallFunction|Explode))

(event Custom|Explode
  (Components|Activation|Activate (Variables|Default|GetNiagara) false)
  (Niagara|SpawnSystematLocation "/Game/Vefects/Free_Fire/Shared/Particles/NS_Fire_Big_Smoke.NS_Fire_Big_Smoke" (Transformation|GetActorLocation))
  (Game|Damage|ApplyRadialDamage (Variables|Default|GetBase%20Damage) (Transformation|GetActorLocation) (Variables|Default|GetDamage%20Radius) 0 (Utilities|Array|MakeArray (Variables|Default|GetGrenadeOwner)) 0 0 false "ECC_Visibility")
  (Components|Activation|Deactivate (Variables|Default|GetNiagara))
  (Actor|DestroyActor))

(fn ConstructionScript)