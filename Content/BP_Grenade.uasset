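; BP_Grenade is a timed grenade actor that explodes shortly after it spawns.
; BeginPlay waits a one-second fuse, then calls Explode.
; Explode spawns a Niagara fire-and-smoke effect at the actor's location, applies radial damage that ignores the GrenadeOwner, and destroys the actor.
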(event Custom|Explode
  (Niagara|SpawnSystematLocation "/Game/Vefects/Free_Fire/Shared/Particles/NS_Fire_Big_Smoke.NS_Fire_Big_Smoke" (Transformation|GetActorLocation))
  (Game|Damage|ApplyRadialDamage (Variables|Default|GetBase%20Damage) (Transformation|GetActorLocation) (Variables|Default|GetDamage%20Radius) 0 (Utilities|Array|MakeArray (Variables|Default|GetGrenadeOwner)) 0 0 false "ECC_Visibility")
  (Actor|DestroyActor))

(event EventBeginPlay
  (Utilities|FlowControl|Delay 1.0)
  (CallFunction|Explode))

(fn ConstructionScript)